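; Player-controlled Paper2D bird for a Flappy-style game, driven by the GM_Flappy game state.
; A looping timeline bobs the bird until the first Jump press starts the game; each jump resets velocity, applies an upward impulse and briefly plays the flap flipbook.
; Tick applies manual gravity once started and pitches the sprite from vertical velocity.
; DeathEvent sets the Death state, then after a delay pauses and shows game over.
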(event Custom|JumpEvent
  (bind _charactermovement (Variables|Character|GetCharacterMovement))
  (bind _bird (Variables|Default|GetBird))
  (bind _bird_2 (Variables|Default|GetBird))
  (Audio|PlaySound2D "/Game/Blueprints/Sounds/Cues/wing_Cue.wing_Cue" 1.0 1.0 0.0 0 0)
  (Components|Movement|StopMovementImmediately _charactermovement)
  (Physics|AddImpulse _charactermovement "0.000000,0.000000,550000.000000" false)
  (Sprite|SetFlipbook _bird_2 "/Game/Blueprints/Resources/Sprites/Flap.Flap")
  (Components|Timeline|SetPlaybackPosition _bird_2 0.0 false)
  (Components|Timeline|SetPlayRate _bird_2 1.0)
  (Utilities|FlowControl|Delay 0.25)
  (Sprite|SetFlipbook _bird "/Game/Blueprints/Resources/Sprites/Idle.Idle")
  (Components|Timeline|SetPlaybackPosition _bird 0.0 false)
  (Components|Timeline|SetPlayRate _bird 0.0))

(event Custom|DeathEvent
  (Audio|PlaySound2D "/Game/Blueprints/Sounds/Cues/die_Cue.die_Cue" 1.0 1.0 0.0 0 0)
  (Variables|/Game/Blueprints/GM_Flappy.GM_Flappy_C|SetGame_State (Variables|Default|GetGame%20Mode%20Ref) "NewEnumerator2")
  (Components|Movement|StopMovementImmediately (Variables|Character|GetCharacterMovement))
  (bind _returnvalue (UserInterface|CreateWidget "/Game/Blueprints/Hud/DeathClass.DeathClass_C"))
  (UserInterface|Viewport|AddtoViewport _returnvalue 0)
  (Utilities|FlowControl|Delay 1.0)
  (Game|SetGamePaused true)
  (Input|DisableInput (Game|GetPlayerController 0))
  (Widget|RemovefromParent (Variables|/Game/Blueprints/GM_Flappy.GM_Flappy_C|GetHud_Ref (Variables|Default|GetGame%20Mode%20Ref)))
  (bind _returnvalue_2 (UserInterface|CreateWidget "/Game/Blueprints/Hud/GameOver.GameOver_C" 0 (Variables|Default|GetGame%20Mode%20Ref)))
  (UserInterface|Viewport|AddtoViewport _returnvalue_2 0))

(event Custom|IdleMovement
  (bind _capsulecomponent (Variables|Collision|GetCapsuleComponent))
  (bind _returnvalue (Transformation|GetWorldLocation _capsulecomponent))
  (bind _newtrack_0 (Timeline|Idle_TL PlayFromStart)
    (:Update
      (Transformation|SetWorldLocation _capsulecomponent (Math|Vector|MakeVector (.x _returnvalue) (.y _returnvalue) (Math|Float|Lerp 0.0 1e+02 _newtrack_0)) false false))
    (:Finished
      (CallFunction|IdleMovement))))

(event Custom|StopIdleMovement
  (bind _capsulecomponent (Variables|Collision|GetCapsuleComponent))
  (bind _returnvalue (Transformation|GetWorldLocation _capsulecomponent))
  (bind _newtrack_0 (Timeline|Idle_TL Stop)
    (:Update
      (Transformation|SetWorldLocation _capsulecomponent (Math|Vector|MakeVector (.x _returnvalue) (.y _returnvalue) (Math|Float|Lerp 0.0 1e+02 _newtrack_0)) false false))
    (:Finished
      (CallFunction|IdleMovement))))

(event EventTick
  (params (DeltaSeconds :type Float%20%28single-precision%29))
  (CallFunction|Gravity)
  (CallFunction|SetRotation))

(event EventBeginPlay
  (bind _returnvalue (Game|GetGameMode))
  (Utilities|IsValid _returnvalue :!label _label
    (:Is%20Valid
      (bind _asgm_flappy (Utilities|Casting|CastToGM_Flappy _returnvalue))
      (Variables|Default|SetGame%20Mode%20Ref _asgm_flappy)
      (CallFunction|IdleMovement))
    (:Is%20Not%20Valid
      (Utilities|FlowControl|DelayUntilNextTick)
      (goto _label))))

(event Input|ActionEvents|InputActionJump
  (params (Key :type Key%20Structure :default "None"))
  (:Pressed
    (if (Utilities|Enum|Equal(Enum) (Variables|/Game/Blueprints/GM_Flappy.GM_Flappy_C|GetGame_State (Variables|Default|GetGame%20Mode%20Ref)) "NewEnumerator1")
      (CallFunction|JumpEvent)
      (else
        (Utilities|FlowControl|DoOnce false
          (:Completed
            (Default|StartGame (Variables|Default|GetGame%20Mode%20Ref))
            (CallFunction|JumpEvent)
            (CallFunction|StopIdleMovement)))))))

(fn ConstructionScript)

(fn Gravity
  (if (Utilities|Enum|NotEqual(Enum) (Variables|/Game/Blueprints/GM_Flappy.GM_Flappy_C|GetGame_State (Variables|Default|GetGame%20Mode%20Ref)) "NewEnumerator0")
    (Physics|AddForce (Variables|Character|GetCharacterMovement) "0.000000,0.000000,-2000000.000000")))

(fn SetRotation
  (bind _charactermovement (Variables|Character|GetCharacterMovement))
  (bind _velocity (Variables|/Script/Engine.MovementComponent|GetVelocity _charactermovement))
  (switch Utilities|FlowControl|Switch|SwitchonGameStateEnum (Variables|/Game/Blueprints/GM_Flappy.GM_Flappy_C|GetGame_State (Variables|Default|GetGame%20Mode%20Ref))
    (:NewEnumerator1
      (Transformation|SetRelativeRotation (Variables|Default|GetBird) (Math|Rotator|MakeRotator 0.0 (Math|Float|MapRangeClamped (.z _velocity) -5e+03 -1e+04 3e+01 -9e+01) 0.0) false false))
    (:NewEnumerator2
      (Transformation|SetRelativeRotation (Variables|Default|GetBird) (Math|Rotator|MakeRotator 0.0 (Math|Float|MapRangeClamped (.z _velocity) 0.0 -2.5e+03 0.0 -9e+01) 0.0) false false))))