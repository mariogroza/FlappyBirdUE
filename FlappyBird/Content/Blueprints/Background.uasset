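; Background actor for a Flappy Bird-style game that kills the player bird when it overlaps the upper or lower death collision.
; On BeginPlay it retries each tick until the game mode is valid, then caches it as GM_Flappy.
; Each overlap calls the bird's DeathEvent only while the game mode's GameState matches one specific enum state.
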(event OnComponentBeginOverlap(DeathCollisionLower)
  (params (OverlappedComponent :type Primitive%20Component%20Object%20Reference) (OtherActor :type Actor%20Object%20Reference) (OtherComp :type Primitive%20Component%20Object%20Reference) (OtherBodyIndex :type Integer) (bFromSweep :type Boolean) (SweepResult :type Hit%20Result%20Structure%20%28by%20ref%29))
  (bind _asplayer_bird (Utilities|Casting|CastToPlayer_Bird OtherActor))
  (if (Utilities|Enum|Equal(Enum) (Variables|/Game/Blueprints/GM_Flappy.GM_Flappy_C|GetGame_State (Variables|Default|GetGameMode_Ref)) "NewEnumerator1")
    (Default|DeathEvent _asplayer_bird)))

(event OnComponentBeginOverlap(DeathCollisionUpper)
  (params (OverlappedComponent :type Primitive%20Component%20Object%20Reference) (OtherActor :type Actor%20Object%20Reference) (OtherComp :type Primitive%20Component%20Object%20Reference) (OtherBodyIndex :type Integer) (bFromSweep :type Boolean) (SweepResult :type Hit%20Result%20Structure%20%28by%20ref%29))
  (bind _asplayer_bird (Utilities|Casting|CastToPlayer_Bird OtherActor))
  (if (Utilities|Enum|Equal(Enum) (Variables|/Game/Blueprints/GM_Flappy.GM_Flappy_C|GetGame_State (Variables|Default|GetGameMode_Ref)) "NewEnumerator1")
    (Default|DeathEvent _asplayer_bird)))

(event EventBeginPlay
  (bind _returnvalue (Game|GetGameMode))
  (Utilities|IsValid _returnvalue :!label _label
    (:Is%20Valid
      (bind _asgm_flappy (Utilities|Casting|CastToGM_Flappy _returnvalue))
      (Variables|Default|SetGameMode_Ref _asgm_flappy))
    (:Is%20Not%20Valid
      (Utilities|FlowControl|DelayUntilNextTick)
      (goto _label))))

(fn ConstructionScript)