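; Game mode for a Flappy Bird-style game that starts play and spawns pipe obstacles.
; StartGame switches the game state, creates and displays the game HUD, and starts a looping timer that calls SpawnPipe at the spawn cooldown interval.
; SpawnPipe always spawns a Pipes actor at the configured X and Y with a random Z height, passing the game mode reference to it, as is done for the HUD.
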(event Custom|StartGame
  (Variables|Default|SetGame_State "NewEnumerator1")
  (bind _returnvalue (UserInterface|CreateWidget "/Game/Blueprints/Hud/GameHud.GameHud_C" 0 self))
  (bind _output_get (Variables|Default|SetHud_Ref _returnvalue))
  (UserInterface|Viewport|AddtoViewport _output_get 0)
  (Utilities|Time|SetTimerbyFunctionName 0 "SpawnPipe" (Variables|Default|GetSpawnCD) true))

(event EventBeginPlay)

(fn ConstructionScript)

(fn SpawnPipe
  (bind _pipespawnlocation (Variables|Default|GetPipeSpawnLocation))
  (Game|SpawnActorfromClass "/Game/Blueprints/Pipes.Pipes_C" (Math|Transform|MakeTransform (Math|Vector|MakeVector (.x _pipespawnlocation) (.y _pipespawnlocation) (Math|Random|RandomFloatinRange -1.3e+03 1.3e+03)) "0, 0, 0" "1.000000,1.000000,1.000000") "AlwaysSpawn" "MultiplyWithRoot" 0 self 0))